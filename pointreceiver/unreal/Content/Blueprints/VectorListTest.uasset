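; Test Blueprint that visualizes a Live Link vector list as mesh instances.
; Each tick it clears the Positions instances, evaluates TargetSubject with VectorListRole, and adds an unrotated, unit-scale instance in local space at every vector of a valid frame.
; The same loop records the highest-Z vector in MaxZVector, which is reset each tick and not read elsewhere in the graph.
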(event EventBeginPlay)

(event Collision|EventActorBeginOverlap
  (params (OtherActor :type Actor%20Object%20Reference)))

(event EventTick
  (params (DeltaSeconds :type Float%20%28single-precision%29))
  (Utilities|FlowControl|Sequence
    (:then_0
      (Components|InstancedStaticMesh|ClearInstances (Variables|Default|GetPositions))
      (Variables|Default|SetMaxZVector "0.000000,0.000000,-100000000000000000.000000"))
    (:then_1
      (bind _dataresult (|EvaluateLiveLinkFramewithSpecificRole (Variables|Default|GetTargetSubject) "/Script/PointreceiverPlugin.VectorListRole")
        (:then
          (bind _array_element (Utilities|Array|ForEachLoopwithBreak (.Vectors (Utilities|Struct|BreakVectorListFrameData (.FrameData (Utilities|Struct|BreakVectorListBlueprintData _dataresult)))))
            (:LoopBody
              (Utilities|FlowControl|Sequence
                (:then_0
                  (Components|InstancedStaticMesh|AddInstance (Variables|Default|GetPositions) (Math|Transform|MakeTransform _array_element) false))
                (:then_1
                  (if (> (.Z (Math|Vector|BreakVector _array_element)) (.Z (Math|Vector|BreakVector (Variables|Default|GetMaxZVector))))
                    (Variables|Default|SetMaxZVector _array_element)))))))))))

(fn ConstructionScript)