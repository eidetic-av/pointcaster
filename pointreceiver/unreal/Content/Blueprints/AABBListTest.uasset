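; This Blueprint visualizes axis-aligned bounding boxes streamed over Live Link, apparently as a test for Pointcaster AABB list data.
; Each tick it clears the BoundingBox instanced mesh and evaluates the target subject's frame with the Pointcaster AABB list role.
; For each box in a valid frame, it adds a local-space instance at the box center, scaled from its size divided by 100.
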(event EventBeginPlay)

(event Collision|EventActorBeginOverlap
  (params (OtherActor :type Actor%20Object%20Reference)))

(event EventTick
  (params (DeltaSeconds :type Float%20%28single-precision%29))
  (Utilities|FlowControl|Sequence
    (:then_0
      (Components|InstancedStaticMesh|ClearInstances (Variables|Default|GetBoundingBox)))
    (:then_1
      (bind _dataresult (|EvaluateLiveLinkFramewithSpecificRole (Variables|Default|GetTargetSubject) "/Script/PointreceiverPlugin.PointcasterAABBListRole")
        (:then
          (bind _array_element (Utilities|Array|ForEachLoopwithBreak (.AABBList (Utilities|Struct|BreakPointcasterAABBListFrameData (.FrameData (Utilities|Struct|BreakPointcasterAABBListBlueprintData _dataresult)))))
            (:LoopBody
              (Utilities|FlowControl|Sequence
                (:then_0
                  (bind _returnvalue (Class|PointcasterAABBFunctionLibrary|GetAABBCenter _array_element)))
                (:then_1
                  (bind _returnvalue_2 (Class|PointcasterAABBFunctionLibrary|GetAABBSize _array_element)))
                (:then_2
                  (Components|InstancedStaticMesh|AddInstance (Variables|Default|GetBoundingBox) (Math|Transform|MakeTransform _returnvalue "0, 0, 0" (/ _returnvalue_2 "100.000000,100.000000,100.000000")) false))))))))))

(fn ConstructionScript)