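; LiveLinkAABBController drives its owning actor, presumably an AABB box, from Live Link data.
; On BeginPlay it puts a dynamic instance of BoxMaterial on the owner's static mesh.
; Each tick it sets that material red, optionally maps a Basic-role subject's first property to opacity within OpacityMinMax, and applies a Transform-role subject to the owner.
; Incoming transforms can also be printed to the log.
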(event EventBeginPlay
  (bind _returnvalue (Rendering|Material|CreateDynamicMaterialInstance (Variables|Default|GetBox%20Material) "None" "None" :!class /Script/Engine.KismetMaterialLibrary))
  (Rendering|Material|SetMaterial (Actor|GetComponentbyClass (Components|GetOwner) "/Script/Engine.StaticMeshComponent") 0 _returnvalue))

(event EventTick
  (params (DeltaSeconds :type Float%20%28single-precision%29))
  (bind _opacity_minmax (Variables|Default|GetOpacity%20MinMax))
  (bind (_x _y) (Math|Vector2D|BreakVector2D _opacity_minmax))
  (Utilities|FlowControl|Sequence
    (:then_0
      (Rendering|Material|SetVectorParameterValue (stale EventBeginPlay _returnvalue) "Color" "(R=1.000000,G=0.000000,B=0.000000,A=1.000000)" :!class /Script/Engine.MaterialInstanceDynamic))
    (:then_1
      (if (Variables|Default|GetSet%20Opacity%20From%20Subject)
        (bind _dataresult (|EvaluateLiveLinkFramewithSpecificRole (Variables|Default|GetOpacity%20Subject) "/Script/LiveLinkInterface.LiveLinkBasicRole")
          (:then
            (Rendering|Material|SetScalarParameterValue (stale EventBeginPlay _returnvalue) "Opacity" (Math|Float|MapRangeClamped (Utilities|Array|Get(acopy) (.PropertyValues (Utilities|Struct|BreakLiveLinkBaseFrameData (.FrameData (Utilities|Struct|BreakLiveLinkBasicBlueprintData _dataresult))))) 0.0 1.0 _x _y) :!class /Script/Engine.MaterialInstanceDynamic)))))
    (:then_2
      (bind _dataresult_2 (|EvaluateLiveLinkFramewithSpecificRole (Variables|Default|GetTransform%20Subject) "/Script/LiveLinkInterface.LiveLinkTransformRole")
        (:then
          (Utilities|FlowControl|Sequence
            (:then_0
              (Transformation|SetActorTransform (Components|GetOwner) (.Transform (Utilities|Struct|BreakLiveLinkTransformFrameData (.FrameData (Utilities|Struct|BreakLiveLinkTransformBlueprintData _dataresult_2))))))
            (:then_1
              (Development|PrintString (Utilities|String|ToString(Transform) (.Transform (Utilities|Struct|BreakLiveLinkTransformFrameData (.FrameData (Utilities|Struct|BreakLiveLinkTransformBlueprintData _dataresult_2))))) false (Variables|Default|GetLog%20Incoming)))))))))