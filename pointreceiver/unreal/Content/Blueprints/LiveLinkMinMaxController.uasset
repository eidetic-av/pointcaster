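; Component that fits its owning actor to a box streamed over Live Link as six normalized min/max axis subjects.
; Each Tick it reorders axes (Y,Z,X to X,Y,Z) and clamp-maps the values into a volume defined by a Live Link transform's location and scale.
; The actor gets the corners' midpoint as location, min minus max as scale, and zero rotation.
; LogIncoming optionally logs the resulting transform.
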(event EventTick
  (params (DeltaSeconds :type Float%20%28single-precision%29))
  (Utilities|FlowControl|Sequence
    (:then_0
      (bind _dataresult (|EvaluateLiveLinkFramewithSpecificRole (Variables|Default|GetSubject%20MinX) "/Script/LiveLinkInterface.LiveLinkBasicRole")))
    (:then_1
      (bind _dataresult_2 (|EvaluateLiveLinkFramewithSpecificRole (Variables|Default|GetSubject%20MinY) "/Script/LiveLinkInterface.LiveLinkBasicRole")))
    (:then_2
      (bind _dataresult_3 (|EvaluateLiveLinkFramewithSpecificRole (Variables|Default|GetSubject%20MinZ) "/Script/LiveLinkInterface.LiveLinkBasicRole")))
    (:then_3
      (Utilities|FlowControl|Sequence
        (:then_0
          (bind _dataresult_4 (|EvaluateLiveLinkFramewithSpecificRole (Variables|Default|GetSubject%20MaxX) "/Script/LiveLinkInterface.LiveLinkBasicRole")))
        (:then_1
          (bind _dataresult_5 (|EvaluateLiveLinkFramewithSpecificRole (Variables|Default|GetSubject%20MaxY) "/Script/LiveLinkInterface.LiveLinkBasicRole")))
        (:then_2
          (bind _dataresult_6 (|EvaluateLiveLinkFramewithSpecificRole (Variables|Default|GetSubject%20MaxZ) "/Script/LiveLinkInterface.LiveLinkBasicRole")))
        (:then_3
          (bind _dataresult_7 (|EvaluateLiveLinkFramewithSpecificRole (Variables|Default|GetSubject%20Transform) "/Script/LiveLinkInterface.LiveLinkTransformRole")))
        (:then_5
          (Utilities|FlowControl|Sequence
            (:then_0
              (Transformation|SetActorTransform (Components|GetOwner) (Math|Transform|MakeTransform (/ (+ (Math|Vector|MakeVector (Math|Float|MapRangeClamped (.X (Math|Vector|BreakVector (Math|Vector|MakeVector (.Y (Math|Vector|BreakVector (Math|Vector|MakeVector (Utilities|Array|Get(acopy) (.PropertyValues (Utilities|Struct|BreakLiveLinkBaseFrameData (.FrameData (Utilities|Struct|BreakLiveLinkBasicBlueprintData _dataresult))))) (Utilities|Array|Get(acopy) (.PropertyValues (Utilities|Struct|BreakLiveLinkBaseFrameData (.FrameData (Utilities|Struct|BreakLiveLinkBasicBlueprintData _dataresult_2))))) (Utilities|Array|Get(acopy) (.PropertyValues (Utilities|Struct|BreakLiveLinkBaseFrameData (.FrameData (Utilities|Struct|BreakLiveLinkBasicBlueprintData _dataresult_3)))))))) (.Z (Math|Vector|BreakVector (Math|Vector|MakeVector (Utilities|Array|Get(acopy) (.PropertyValues (Utilities|Struct|BreakLiveLinkBaseFrameData (.FrameData (Utilities|Struct|BreakLiveLinkBasicBlueprintData _dataresult))))) (Utilities|Array|Get(acopy) (.PropertyValues (Utilities|Struct|BreakLiveLinkBaseFrameData (.FrameData (Utilities|Struct|BreakLiveLinkBasicBlueprintData _dataresult_2))))) (Utilities|Array|Get(acopy) (.PropertyValues (Utilities|Struct|BreakLiveLinkBaseFrameData (.FrameData (Utilities|Struct|BreakLiveLinkBasicBlueprintData _dataresult_3)))))))) (.X (Math|Vector|BreakVector (Math|Vector|MakeVector (Utilities|Array|Get(acopy) (.PropertyValues (Utilities|Struct|BreakLiveLinkBaseFrameData (.FrameData (Utilities|Struct|BreakLiveLinkBasicBlueprintData _dataresult))))) (Utilities|Array|Get(acopy) (.PropertyValues (Utilities|Struct|BreakLiveLinkBaseFrameData (.FrameData (Utilities|Struct|BreakLiveLinkBasicBlueprintData _dataresult_2))))) (Utilities|Array|Get(acopy) (.PropertyValues (Utilities|Struct|BreakLiveLinkBaseFrameData (.FrameData (Utilities|Struct|BreakLiveLinkBasicBlueprintData _dataresult_3))))))))))) 0.0 1.0 (.X (Math|Vector|BreakVector (- (.Location (Math|Transform|BreakTransform (.Transform (Utilities|Struct|BreakLiveLinkTransformFrameData (.FrameData (Utilities|Struct|BreakLiveLinkTransformBlueprintData _dataresult_7)))))) (* (.Scale (Math|Transform|BreakTransform (.Transform (Utilities|Struct|BreakLiveLinkTransformFrameData (.FrameData (Utilities|Struct|BreakLiveLinkTransformBlueprintData _dataresult_7)))))) "0.500000,0.500000,0.500000")))) (.X (Math|Vector|BreakVector (+ (.Location (Math|Transform|BreakTransform (.Transform (Utilities|Struct|BreakLiveLinkTransformFrameData (.FrameData (Utilities|Struct|BreakLiveLinkTransformBlueprintData _dataresult_7)))))) (* (.Scale (Math|Transform|BreakTransform (.Transform (Utilities|Struct|BreakLiveLinkTransformFrameData (.FrameData (Utilities|Struct|BreakLiveLinkTransformBlueprintData _dataresult_7)))))) "0.500000,0.500000,0.500000"))))) (Math|Float|MapRangeClamped (.Y (Math|Vector|BreakVector (Math|Vector|MakeVector (.Y (Math|Vector|BreakVector (Math|Vector|MakeVector (Utilities|Array|Get(acopy) (.PropertyValues (Utilities|Struct|BreakLiveLinkBaseFrameData (.FrameData (Utilities|Struct|BreakLiveLinkBasicBlueprintData _dataresult))))) (Utilities|Array|Get(acopy) (.PropertyValues (Utilities|Struct|BreakLiveLinkBaseFrameData (.FrameData (Utilities|Struct|BreakLiveLinkBasicBlueprintData _dataresult_2))))) (Utilities|Array|Get(acopy) (.PropertyValues (Utilities|Struct|BreakLiveLinkBaseFrameData (.FrameData (Utilities|Struct|BreakLiveLinkBasicBlueprintData _dataresult_3)))))))) (.Z (Math|Vector|BreakVector (Math|Vector|MakeVector (Utilities|Array|Get(acopy) (.PropertyValues (Utilities|Struct|BreakLiveLinkBaseFrameData (.FrameData (Utilities|Struct|BreakLiveLinkBasicBlueprintData _dataresult))))) (Utilities|Array|Get(acopy) (.PropertyValues (Utilities|Struct|BreakLiveLinkBaseFrameData (.FrameData (Utilities|Struct|BreakLiveLinkBasicBlueprintData _dataresult_2))))) (Utilities|Array|Get(acopy) (.PropertyValues (Utilities|Struct|BreakLiveLinkBaseFrameData (.FrameData (Utilities|Struct|BreakLiveLinkBasicBlueprintData _dataresult_3)))))))) (.X (Math|Vector|BreakVector (Math|Vector|MakeVector (Utilities|Array|Get(acopy) (.PropertyValues (Utilities|Struct|BreakLiveLinkBaseFrameData (.FrameData (Utilities|Struct|BreakLiveLinkBasicBlueprintData _dataresult))))) (Utilities|Array|Get(acopy) (.PropertyValues (Utilities|Struct|BreakLiveLinkBaseFrameData (.FrameData (Utilities|Struct|BreakLiveLinkBasicBlueprintData _dataresult_2))))) (Utilities|Array|Get(acopy) (.PropertyValues (Utilities|Struct|BreakLiveLinkBaseFrameData (.FrameData (Utilities|Struct|BreakLiveLinkBasicBlueprintData _dataresult_3))))))))))) 0.0 1.0 (.Y (Math|Vector|BreakVector (- (.Location (Math|Transform|BreakTransform (.Transform (Utilities|Struct|BreakLiveLinkTransformFrameData (.FrameData (Utilities|Struct|BreakLiveLinkTransformBlueprintData _dataresult_7)))))) (* (.Scale (Math|Transform|BreakTransform (.Transform (Utilities|Struct|BreakLiveLinkTransformFrameData (.FrameData (Utilities|Struct|BreakLiveLinkTransformBlueprintData _dataresult_7)))))) "0.500000,0.500000,0.500000")))) (.Y (Math|Vector|BreakVector (+ (.Location (Math|Transform|BreakTransform (.Transform (Utilities|Struct|BreakLiveLinkTransformFrameData (.FrameData (Utilities|Struct|BreakLiveLinkTransformBlueprintData _dataresult_7)))))) (* (.Scale (Math|Transform|BreakTransform (.Transform (Utilities|Struct|BreakLiveLinkTransformFrameData (.FrameData (Utilities|Struct|BreakLiveLinkTransformBlueprintData _dataresult_7)))))) "0.500000,0.500000,0.500000"))))) (Math|Float|MapRangeClamped (.Z (Math|Vector|BreakVector (Math|Vector|MakeVector (.Y (Math|Vector|BreakVector (Math|Vector|MakeVector (Utilities|Array|Get(acopy) (.PropertyValues (Utilities|Struct|BreakLiveLinkBaseFrameData (.FrameData (Utilities|Struct|BreakLiveLinkBasicBlueprintData _dataresult))))) (Utilities|Array|Get(acopy) (.PropertyValues (Utilities|Struct|BreakLiveLinkBaseFrameData (.FrameData (Utilities|Struct|BreakLiveLinkBasicBlueprintData _dataresult_2))))) (Utilities|Array|Get(acopy) (.PropertyValues (Utilities|Struct|BreakLiveLinkBaseFrameData (.FrameData (Utilities|Struct|BreakLiveLinkBasicBlueprintData _dataresult_3)))))))) (.Z (Math|Vector|BreakVector (Math|Vector|MakeVector (Utilities|Array|Get(acopy) (.PropertyValues (Utilities|Struct|BreakLiveLinkBaseFrameData (.FrameData (Utilities|Struct|BreakLiveLinkBasicBlueprintData _dataresult))))) (Utilities|Array|Get(acopy) (.PropertyValues (Utilities|Struct|BreakLiveLinkBaseFrameData (.FrameData (Utilities|Struct|BreakLiveLinkBasicBlueprintData _dataresult_2))))) (Utilities|Array|Get(acopy) (.PropertyValues (Utilities|Struct|BreakLiveLinkBaseFrameData (.FrameData (Utilities|Struct|BreakLiveLinkBasicBlueprintData _dataresult_3)))))))) (.X (Math|Vector|BreakVector (Math|Vector|MakeVector (Utilities|Array|Get(acopy) (.PropertyValues (Utilities|Struct|BreakLiveLinkBaseFrameData (.FrameData (Utilities|Struct|BreakLiveLinkBasicBlueprintData _dataresult))))) (Utilities|Array|Get(acopy) (.PropertyValues (Utilities|Struct|BreakLiveLinkBaseFrameData (.FrameData (Utilities|Struct|BreakLiveLinkBasicBlueprintData _dataresult_2))))) (Utilities|Array|Get(acopy) (.PropertyValues (Utilities|Struct|BreakLiveLinkBaseFrameData (.FrameData (Utilities|Struct|BreakLiveLinkBasicBlueprintData _dataresult_3))))))))))) 0.0 1.0 (.Z (Math|Vector|BreakVector (- (.Location (Math|Transform|BreakTransform (.Transform (Utilities|Struct|BreakLiveLinkTransformFrameData (.FrameData (Utilities|Struct|BreakLiveLinkTransformBlueprintData _dataresult_7)))))) (* (.Scale (Math|Transform|BreakTransform (.Transform (Utilities|Struct|BreakLiveLinkTransformFrameData (.FrameData (Utilities|Struct|BreakLiveLinkTransformBlueprintData _dataresult_7)))))) "0.500000,0.500000,0.500000")))) (.Z (Math|Vector|BreakVector (+ (.Location (Math|Transform|BreakTransform (.Transform (Utilities|Struct|BreakLiveLinkTransformFrameData (.FrameData (Utilities|Struct|BreakLiveLinkTransformBlueprintData _dataresult_7)))))) (* (.Scale (Math|Transform|BreakTransform (.Transform (Utilities|Struct|BreakLiveLinkTransformFrameData (.FrameData (Utilities|Struct|BreakLiveLinkTransformBlueprintData _dataresult_7)))))) "0.500000,0.500000,0.500000")))))) (Math|Vector|MakeVector (Math|Float|MapRangeClamped (.X (Math|Vector|BreakVector (Math|Vector|MakeVector (.Y (Math|Vector|BreakVector (Math|Vector|MakeVector (Utilities|Array|Get(acopy) (.PropertyValues (Utilities|Struct|BreakLiveLinkBaseFrameData (.FrameData (Utilities|Struct|BreakLiveLinkBasicBlueprintData _dataresult_4))))) (Utilities|Array|Get(acopy) (.PropertyValues (Utilities|Struct|BreakLiveLinkBaseFrameData (.FrameData (Utilities|Struct|BreakLiveLinkBasicBlueprintData _dataresult_5))))) (Utilities|Array|Get(acopy) (.PropertyValues (Utilities|Struct|BreakLiveLinkBaseFrameData (.FrameData (Utilities|Struct|BreakLiveLinkBasicBlueprintData _dataresult_6)))))))) (.Z (Math|Vector|BreakVector (Math|Vector|MakeVector (Utilities|Array|Get(acopy) (.PropertyValues (Utilities|Struct|BreakLiveLinkBaseFrameData (.FrameData (Utilities|Struct|BreakLiveLinkBasicBlueprintData _dataresult_4))))) (Utilities|Array|Get(acopy) (.PropertyValues (Utilities|Struct|BreakLiveLinkBaseFrameData (.FrameData (Utilities|Struct|BreakLiveLinkBasicBlueprintData _dataresult_5))))) (Utilities|Array|Get(acopy) (.PropertyValues (Utilities|Struct|BreakLiveLinkBaseFrameData (.FrameData (Utilities|Struct|BreakLiveLinkBasicBlueprintData _dataresult_6)))))))) (.X (Math|Vector|BreakVector (Math|Vector|MakeVector (Utilities|Array|Get(acopy) (.PropertyValues (Utilities|Struct|BreakLiveLinkBaseFrameData (.FrameData (Utilities|Struct|BreakLiveLinkBasicBlueprintData _dataresult_4))))) (Utilities|Array|Get(acopy) (.PropertyValues (Utilities|Struct|BreakLiveLinkBaseFrameData (.FrameData (Utilities|Struct|BreakLiveLinkBasicBlueprintData _dataresult_5))))) (Utilities|Array|Get(acopy) (.PropertyValues (Utilities|Struct|BreakLiveLinkBaseFrameData (.FrameData (Utilities|Struct|BreakLiveLinkBasicBlueprintData _dataresult_6))))))))))) 0.0 1.0 (.X (Math|Vector|BreakVector (- (.Location (Math|Transform|BreakTransform (.Transform (Utilities|Struct|BreakLiveLinkTransformFrameData (.FrameData (Utilities|Struct|BreakLiveLinkTransformBlueprintData _dataresult_7)))))) (* (.Scale (Math|Transform|BreakTransform (.Transform (Utilities|Struct|BreakLiveLinkTransformFrameData (.FrameData (Utilities|Struct|BreakLiveLinkTransformBlueprintData _dataresult_7)))))) "0.500000,0.500000,0.500000")))) (.X (Math|Vector|BreakVector (+ (.Location (Math|Transform|BreakTransform (.Transform (Utilities|Struct|BreakLiveLinkTransformFrameData (.FrameData (Utilities|Struct|BreakLiveLinkTransformBlueprintData _dataresult_7)))))) (* (.Scale (Math|Transform|BreakTransform (.Transform (Utilities|Struct|BreakLiveLinkTransformFrameData (.FrameData (Utilities|Struct|BreakLiveLinkTransformBlueprintData _dataresult_7)))))) "0.500000,0.500000,0.500000"))))) (Math|Float|MapRangeClamped (.Y (Math|Vector|BreakVector (Math|Vector|MakeVector (.Y (Math|Vector|BreakVector (Math|Vector|MakeVector (Utilities|Array|Get(acopy) (.PropertyValues (Utilities|Struct|BreakLiveLinkBaseFrameData (.FrameData (Utilities|Struct|BreakLiveLinkBasicBlueprintData _dataresult_4))))) (Utilities|Array|Get(acopy) (.PropertyValues (Utilities|Struct|BreakLiveLinkBaseFrameData (.FrameData (Utilities|Struct|BreakLiveLinkBasicBlueprintData _dataresult_5))))) (Utilities|Array|Get(acopy) (.PropertyValues (Utilities|Struct|BreakLiveLinkBaseFrameData (.FrameData (Utilities|Struct|BreakLiveLinkBasicBlueprintData _dataresult_6)))))))) (.Z (Math|Vector|BreakVector (Math|Vector|MakeVector (Utilities|Array|Get(acopy) (.PropertyValues (Utilities|Struct|BreakLiveLinkBaseFrameData (.FrameData (Utilities|Struct|BreakLiveLinkBasicBlueprintData _dataresult_4))))) (Utilities|Array|Get(acopy) (.PropertyValues (Utilities|Struct|BreakLiveLinkBaseFrameData (.FrameData (Utilities|Struct|BreakLiveLinkBasicBlueprintData _dataresult_5))))) (Utilities|Array|Get(acopy) (.PropertyValues (Utilities|Struct|BreakLiveLinkBaseFrameData (.FrameData (Utilities|Struct|BreakLiveLinkBasicBlueprintData _dataresult_6)))))))) (.X (Math|Vector|BreakVector (Math|Vector|MakeVector (Utilities|Array|Get(acopy) (.PropertyValues (Utilities|Struct|BreakLiveLinkBaseFrameData (.FrameData (Utilities|Struct|BreakLiveLinkBasicBlueprintData _dataresult_4))))) (Utilities|Array|Get(acopy) (.PropertyValues (Utilities|Struct|BreakLiveLinkBaseFrameData (.FrameData (Utilities|Struct|BreakLiveLinkBasicBlueprintData _dataresult_5))))) (Utilities|Array|Get(acopy) (.PropertyValues (Utilities|Struct|BreakLiveLinkBaseFrameData (.FrameData (Utilities|Struct|BreakLiveLinkBasicBlueprintData _dataresult_6))))))))))) 0.0 1.0 (.Y (Math|Vector|BreakVector (- (.Location (Math|Transform|BreakTransform (.Transform (Utilities|Struct|BreakLiveLinkTransformFrameData (.FrameData (Utilities|Struct|BreakLiveLinkTransformBlueprintData _dataresult_7)))))) (* (.Scale (Math|Transform|BreakTransform (.Transform (Utilities|Struct|BreakLiveLinkTransformFrameData (.FrameData (Utilities|Struct|BreakLiveLinkTransformBlueprintData _dataresult_7)))))) "0.500000,0.500000,0.500000")))) (.Y (Math|Vector|BreakVector (+ (.Location (Math|Transform|BreakTransform (.Transform (Utilities|Struct|BreakLiveLinkTransformFrameData (.FrameData (Utilities|Struct|BreakLiveLinkTransformBlueprintData _dataresult_7)))))) (* (.Scale (Math|Transform|BreakTransform (.Transform (Utilities|Struct|BreakLiveLinkTransformFrameData (.FrameData (Utilities|Struct|BreakLiveLinkTransformBlueprintData _dataresult_7)))))) "0.500000,0.500000,0.500000"))))) (Math|Float|MapRangeClamped (.Z (Math|Vector|BreakVector (Math|Vector|MakeVector (.Y (Math|Vector|BreakVector (Math|Vector|MakeVector (Utilities|Array|Get(acopy) (.PropertyValues (Utilities|Struct|BreakLiveLinkBaseFrameData (.FrameData (Utilities|Struct|BreakLiveLinkBasicBlueprintData _dataresult_4))))) (Utilities|Array|Get(acopy) (.PropertyValues (Utilities|Struct|BreakLiveLinkBaseFrameData (.FrameData (Utilities|Struct|BreakLiveLinkBasicBlueprintData _dataresult_5))))) (Utilities|Array|Get(acopy) (.PropertyValues (Utilities|Struct|BreakLiveLinkBaseFrameData (.FrameData (Utilities|Struct|BreakLiveLinkBasicBlueprintData _dataresult_6)))))))) (.Z (Math|Vector|BreakVector (Math|Vector|MakeVector (Utilities|Array|Get(acopy) (.PropertyValues (Utilities|Struct|BreakLiveLinkBaseFrameData (.FrameData (Utilities|Struct|BreakLiveLinkBasicBlueprintData _dataresult_4))))) (Utilities|Array|Get(acopy) (.PropertyValues (Utilities|Struct|BreakLiveLinkBaseFrameData (.FrameData (Utilities|Struct|BreakLiveLinkBasicBlueprintData _dataresult_5))))) (Utilities|Array|Get(acopy) (.PropertyValues (Utilities|Struct|BreakLiveLinkBaseFrameData (.FrameData (Utilities|Struct|BreakLiveLinkBasicBlueprintData _dataresult_6)))))))) (.X (Math|Vector|BreakVector (Math|Vector|MakeVector (Utilities|Array|Get(acopy) (.PropertyValues (Utilities|Struct|BreakLiveLinkBaseFrameData (.FrameData (Utilities|Struct|BreakLiveLinkBasicBlueprintData _dataresult_4))))) (Utilities|Array|Get(acopy) (.PropertyValues (Utilities|Struct|BreakLiveLinkBaseFrameData (.FrameData (Utilities|Struct|BreakLiveLinkBasicBlueprintData _dataresult_5))))) (Utilities|Array|Get(acopy) (.PropertyValues (Utilities|Struct|BreakLiveLinkBaseFrameData (.FrameData (Utilities|Struct|BreakLiveLinkBasicBlueprintData _dataresult_6))))))))))) 0.0 1.0 (.Z (Math|Vector|BreakVector (- (.Location (Math|Transform|BreakTransform (.Transform (Utilities|Struct|BreakLiveLinkTransformFrameData (.FrameData (Utilities|Struct|BreakLiveLinkTransformBlueprintData _dataresult_7)))))) (* (.Scale (Math|Transform|BreakTransform (.Transform (Utilities|Struct|BreakLiveLinkTransformFrameData (.FrameData (Utilities|Struct|BreakLiveLinkTransformBlueprintData _dataresult_7)))))) "0.500000,0.500000,0.500000")))) (.Z (Math|Vector|BreakVector (+ (.Location (Math|Transform|BreakTransform (.Transform (Utilities|Struct|BreakLiveLinkTransformFrameData (.FrameData (Utilities|Struct|BreakLiveLinkTransformBlueprintData _dataresult_7)))))) (* (.Scale (Math|Transform|BreakTransform (.Transform (Utilities|Struct|BreakLiveLinkTransformFrameData (.FrameData (Utilities|Struct|BreakLiveLinkTransformBlueprintData _dataresult_7)))))) "0.500000,0.500000,0.500000"))))))) "2.000000,2.000000,2.000000") "0, 0, 0" (- (Math|Vector|MakeVector (Math|Float|MapRangeClamped (.X (Math|Vector|BreakVector (Math|Vector|MakeVector (.Y (Math|Vector|BreakVector (Math|Vector|MakeVector (Utilities|Array|Get(acopy) (.PropertyValues (Utilities|Struct|BreakLiveLinkBaseFrameData (.FrameData (Utilities|Struct|BreakLiveLinkBasicBlueprintData _dataresult))))) (Utilities|Array|Get(acopy) (.PropertyValues (Utilities|Struct|BreakLiveLinkBaseFrameData (.FrameData (Utilities|Struct|BreakLiveLinkBasicBlueprintData _dataresult_2))))) (Utilities|Array|Get(acopy) (.PropertyValues (Utilities|Struct|BreakLiveLinkBaseFrameData (.FrameData (Utilities|Struct|BreakLiveLinkBasicBlueprintData _dataresult_3)))))))) (.Z (Math|Vector|BreakVector (Math|Vector|MakeVector (Utilities|Array|Get(acopy) (.PropertyValues (Utilities|Struct|BreakLiveLinkBaseFrameData (.FrameData (Utilities|Struct|BreakLiveLinkBasicBlueprintData _dataresult))))) (Utilities|Array|Get(acopy) (.PropertyValues (Utilities|Struct|BreakLiveLinkBaseFrameData (.FrameData (Utilities|Struct|BreakLiveLinkBasicBlueprintData _dataresult_2))))) (Utilities|Array|Get(acopy) (.PropertyValues (Utilities|Struct|BreakLiveLinkBaseFrameData (.FrameData (Utilities|Struct|BreakLiveLinkBasicBlueprintData _dataresult_3)))))))) (.X (Math|Vector|BreakVector (Math|Vector|MakeVector (Utilities|Array|Get(acopy) (.PropertyValues (Utilities|Struct|BreakLiveLinkBaseFrameData (.FrameData (Utilities|Struct|BreakLiveLinkBasicBlueprintData _dataresult))))) (Utilities|Array|Get(acopy) (.PropertyValues (Utilities|Struct|BreakLiveLinkBaseFrameData (.FrameData (Utilities|Struct|BreakLiveLinkBasicBlueprintData _dataresult_2))))) (Utilities|Array|Get(acopy) (.PropertyValues (Utilities|Struct|BreakLiveLinkBaseFrameData (.FrameData (Utilities|Struct|BreakLiveLinkBasicBlueprintData _dataresult_3))))))))))) 0.0 1.0 (.X (Math|Vector|BreakVector (- (.Location (Math|Transform|BreakTransform (.Transform (Utilities|Struct|BreakLiveLinkTransformFrameData (.FrameData (Utilities|Struct|BreakLiveLinkTransformBlueprintData _dataresult_7)))))) (* (.Scale (Math|Transform|BreakTransform (.Transform (Utilities|Struct|BreakLiveLinkTransformFrameData (.FrameData (Utilities|Struct|BreakLiveLinkTransformBlueprintData _dataresult_7)))))) "0.500000,0.500000,0.500000")))) (.X (Math|Vector|BreakVector (+ (.Location (Math|Transform|BreakTransform (.Transform (Utilities|Struct|BreakLiveLinkTransformFrameData (.FrameData (Utilities|Struct|BreakLiveLinkTransformBlueprintData _dataresult_7)))))) (* (.Scale (Math|Transform|BreakTransform (.Transform (Utilities|Struct|BreakLiveLinkTransformFrameData (.FrameData (Utilities|Struct|BreakLiveLinkTransformBlueprintData _dataresult_7)))))) "0.500000,0.500000,0.500000"))))) (Math|Float|MapRangeClamped (.Y (Math|Vector|BreakVector (Math|Vector|MakeVector (.Y (Math|Vector|BreakVector (Math|Vector|MakeVector (Utilities|Array|Get(acopy) (.PropertyValues (Utilities|Struct|BreakLiveLinkBaseFrameData (.FrameData (Utilities|Struct|BreakLiveLinkBasicBlueprintData _dataresult))))) (Utilities|Array|Get(acopy) (.PropertyValues (Utilities|Struct|BreakLiveLinkBaseFrameData (.FrameData (Utilities|Struct|BreakLiveLinkBasicBlueprintData _dataresult_2))))) (Utilities|Array|Get(acopy) (.PropertyValues (Utilities|Struct|BreakLiveLinkBaseFrameData (.FrameData (Utilities|Struct|BreakLiveLinkBasicBlueprintData _dataresult_3)))))))) (.Z (Math|Vector|BreakVector (Math|Vector|MakeVector (Utilities|Array|Get(acopy) (.PropertyValues (Utilities|Struct|BreakLiveLinkBaseFrameData (.FrameData (Utilities|Struct|BreakLiveLinkBasicBlueprintData _dataresult))))) (Utilities|Array|Get(acopy) (.PropertyValues (Utilities|Struct|BreakLiveLinkBaseFrameData (.FrameData (Utilities|Struct|BreakLiveLinkBasicBlueprintData _dataresult_2))))) (Utilities|Array|Get(acopy) (.PropertyValues (Utilities|Struct|BreakLiveLinkBaseFrameData (.FrameData (Utilities|Struct|BreakLiveLinkBasicBlueprintData _dataresult_3)))))))) (.X (Math|Vector|BreakVector (Math|Vector|MakeVector (Utilities|Array|Get(acopy) (.PropertyValues (Utilities|Struct|BreakLiveLinkBaseFrameData (.FrameData (Utilities|Struct|BreakLiveLinkBasicBlueprintData _dataresult))))) (Utilities|Array|Get(acopy) (.PropertyValues (Utilities|Struct|BreakLiveLinkBaseFrameData (.FrameData (Utilities|Struct|BreakLiveLinkBasicBlueprintData _dataresult_2))))) (Utilities|Array|Get(acopy) (.PropertyValues (Utilities|Struct|BreakLiveLinkBaseFrameData (.FrameData (Utilities|Struct|BreakLiveLinkBasicBlueprintData _dataresult_3))))))))))) 0.0 1.0 (.Y (Math|Vector|BreakVector (- (.Location (Math|Transform|BreakTransform (.Transform (Utilities|Struct|BreakLiveLinkTransformFrameData (.FrameData (Utilities|Struct|BreakLiveLinkTransformBlueprintData _dataresult_7)))))) (* (.Scale (Math|Transform|BreakTransform (.Transform (Utilities|Struct|BreakLiveLinkTransformFrameData (.FrameData (Utilities|Struct|BreakLiveLinkTransformBlueprintData _dataresult_7)))))) "0.500000,0.500000,0.500000")))) (.Y (Math|Vector|BreakVector (+ (.Location (Math|Transform|BreakTransform (.Transform (Utilities|Struct|BreakLiveLinkTransformFrameData (.FrameData (Utilities|Struct|BreakLiveLinkTransformBlueprintData _dataresult_7)))))) (* (.Scale (Math|Transform|BreakTransform (.Transform (Utilities|Struct|BreakLiveLinkTransformFrameData (.FrameData (Utilities|Struct|BreakLiveLinkTransformBlueprintData _dataresult_7)))))) "0.500000,0.500000,0.500000"))))) (Math|Float|MapRangeClamped (.Z (Math|Vector|BreakVector (Math|Vector|MakeVector (.Y (Math|Vector|BreakVector (Math|Vector|MakeVector (Utilities|Array|Get(acopy) (.PropertyValues (Utilities|Struct|BreakLiveLinkBaseFrameData (.FrameData (Utilities|Struct|BreakLiveLinkBasicBlueprintData _dataresult))))) (Utilities|Array|Get(acopy) (.PropertyValues (Utilities|Struct|BreakLiveLinkBaseFrameData (.FrameData (Utilities|Struct|BreakLiveLinkBasicBlueprintData _dataresult_2))))) (Utilities|Array|Get(acopy) (.PropertyValues (Utilities|Struct|BreakLiveLinkBaseFrameData (.FrameData (Utilities|Struct|BreakLiveLinkBasicBlueprintData _dataresult_3)))))))) (.Z (Math|Vector|BreakVector (Math|Vector|MakeVector (Utilities|Array|Get(acopy) (.PropertyValues (Utilities|Struct|BreakLiveLinkBaseFrameData (.FrameData (Utilities|Struct|BreakLiveLinkBasicBlueprintData _dataresult))))) (Utilities|Array|Get(acopy) (.PropertyValues (Utilities|Struct|BreakLiveLinkBaseFrameData (.FrameData (Utilities|Struct|BreakLiveLinkBasicBlueprintData _dataresult_2))))) (Utilities|Array|Get(acopy) (.PropertyValues (Utilities|Struct|BreakLiveLinkBaseFrameData (.FrameData (Utilities|Struct|BreakLiveLinkBasicBlueprintData _dataresult_3)))))))) (.X (Math|Vector|BreakVector (Math|Vector|MakeVector (Utilities|Array|Get(acopy) (.PropertyValues (Utilities|Struct|BreakLiveLinkBaseFrameData (.FrameData (Utilities|Struct|BreakLiveLinkBasicBlueprintData _dataresult))))) (Utilities|Array|Get(acopy) (.PropertyValues (Utilities|Struct|BreakLiveLinkBaseFrameData (.FrameData (Utilities|Struct|BreakLiveLinkBasicBlueprintData _dataresult_2))))) (Utilities|Array|Get(acopy) (.PropertyValues (Utilities|Struct|BreakLiveLinkBaseFrameData (.FrameData (Utilities|Struct|BreakLiveLinkBasicBlueprintData _dataresult_3))))))))))) 0.0 1.0 (.Z (Math|Vector|BreakVector (- (.Location (Math|Transform|BreakTransform (.Transform (Utilities|Struct|BreakLiveLinkTransformFrameData (.FrameData (Utilities|Struct|BreakLiveLinkTransformBlueprintData _dataresult_7)))))) (* (.Scale (Math|Transform|BreakTransform (.Transform (Utilities|Struct|BreakLiveLinkTransformFrameData (.FrameData (Utilities|Struct|BreakLiveLinkTransformBlueprintData _dataresult_7)))))) "0.500000,0.500000,0.500000")))) (.Z (Math|Vector|BreakVector (+ (.Location (Math|Transform|BreakTransform (.Transform (Utilities|Struct|BreakLiveLinkTransformFrameData (.FrameData (Utilities|Struct|BreakLiveLinkTransformBlueprintData _dataresult_7)))))) (* (.Scale (Math|Transform|BreakTransform (.Transform (Utilities|Struct|BreakLiveLinkTransformFrameData (.FrameData (Utilities|Struct|BreakLiveLinkTransformBlueprintData _dataresult_7)))))) "0.500000,0.500000,0.500000")))))) (Math|Vector|MakeVector (Math|Float|MapRangeClamped (.X (Math|Vector|BreakVector (Math|Vector|MakeVector (.Y (Math|Vector|BreakVector (Math|Vector|MakeVector (Utilities|Array|Get(acopy) (.PropertyValues (Utilities|Struct|BreakLiveLinkBaseFrameData (.FrameData (Utilities|Struct|BreakLiveLinkBasicBlueprintData _dataresult_4))))) (Utilities|Array|Get(acopy) (.PropertyValues (Utilities|Struct|BreakLiveLinkBaseFrameData (.FrameData (Utilities|Struct|BreakLiveLinkBasicBlueprintData _dataresult_5))))) (Utilities|Array|Get(acopy) (.PropertyValues (Utilities|Struct|BreakLiveLinkBaseFrameData (.FrameData (Utilities|Struct|BreakLiveLinkBasicBlueprintData _dataresult_6)))))))) (.Z (Math|Vector|BreakVector (Math|Vector|MakeVector (Utilities|Array|Get(acopy) (.PropertyValues (Utilities|Struct|BreakLiveLinkBaseFrameData (.FrameData (Utilities|Struct|BreakLiveLinkBasicBlueprintData _dataresult_4))))) (Utilities|Array|Get(acopy) (.PropertyValues (Utilities|Struct|BreakLiveLinkBaseFrameData (.FrameData (Utilities|Struct|BreakLiveLinkBasicBlueprintData _dataresult_5))))) (Utilities|Array|Get(acopy) (.PropertyValues (Utilities|Struct|BreakLiveLinkBaseFrameData (.FrameData (Utilities|Struct|BreakLiveLinkBasicBlueprintData _dataresult_6)))))))) (.X (Math|Vector|BreakVector (Math|Vector|MakeVector (Utilities|Array|Get(acopy) (.PropertyValues (Utilities|Struct|BreakLiveLinkBaseFrameData (.FrameData (Utilities|Struct|BreakLiveLinkBasicBlueprintData _dataresult_4))))) (Utilities|Array|Get(acopy) (.PropertyValues (Utilities|Struct|BreakLiveLinkBaseFrameData (.FrameData (Utilities|Struct|BreakLiveLinkBasicBlueprintData _dataresult_5))))) (Utilities|Array|Get(acopy) (.PropertyValues (Utilities|Struct|BreakLiveLinkBaseFrameData (.FrameData (Utilities|Struct|BreakLiveLinkBasicBlueprintData _dataresult_6))))))))))) 0.0 1.0 (.X (Math|Vector|BreakVector (- (.Location (Math|Transform|BreakTransform (.Transform (Utilities|Struct|BreakLiveLinkTransformFrameData (.FrameData (Utilities|Struct|BreakLiveLinkTransformBlueprintData _dataresult_7)))))) (* (.Scale (Math|Transform|BreakTransform (.Transform (Utilities|Struct|BreakLiveLinkTransformFrameData (.FrameData (Utilities|Struct|BreakLiveLinkTransformBlueprintData _dataresult_7)))))) "0.500000,0.500000,0.500000")))) (.X (Math|Vector|BreakVector (+ (.Location (Math|Transform|BreakTransform (.Transform (Utilities|Struct|BreakLiveLinkTransformFrameData (.FrameData (Utilities|Struct|BreakLiveLinkTransformBlueprintData _dataresult_7)))))) (* (.Scale (Math|Transform|BreakTransform (.Transform (Utilities|Struct|BreakLiveLinkTransformFrameData (.FrameData (Utilities|Struct|BreakLiveLinkTransformBlueprintData _dataresult_7)))))) "0.500000,0.500000,0.500000"))))) (Math|Float|MapRangeClamped (.Y (Math|Vector|BreakVector (Math|Vector|MakeVector (.Y (Math|Vector|BreakVector (Math|Vector|MakeVector (Utilities|Array|Get(acopy) (.PropertyValues (Utilities|Struct|BreakLiveLinkBaseFrameData (.FrameData (Utilities|Struct|BreakLiveLinkBasicBlueprintData _dataresult_4))))) (Utilities|Array|Get(acopy) (.PropertyValues (Utilities|Struct|BreakLiveLinkBaseFrameData (.FrameData (Utilities|Struct|BreakLiveLinkBasicBlueprintData _dataresult_5))))) (Utilities|Array|Get(acopy) (.PropertyValues (Utilities|Struct|BreakLiveLinkBaseFrameData (.FrameData (Utilities|Struct|BreakLiveLinkBasicBlueprintData _dataresult_6)))))))) (.Z (Math|Vector|BreakVector (Math|Vector|MakeVector (Utilities|Array|Get(acopy) (.PropertyValues (Utilities|Struct|BreakLiveLinkBaseFrameData (.FrameData (Utilities|Struct|BreakLiveLinkBasicBlueprintData _dataresult_4))))) (Utilities|Array|Get(acopy) (.PropertyValues (Utilities|Struct|BreakLiveLinkBaseFrameData (.FrameData (Utilities|Struct|BreakLiveLinkBasicBlueprintData _dataresult_5))))) (Utilities|Array|Get(acopy) (.PropertyValues (Utilities|Struct|BreakLiveLinkBaseFrameData (.FrameData (Utilities|Struct|BreakLiveLinkBasicBlueprintData _dataresult_6)))))))) (.X (Math|Vector|BreakVector (Math|Vector|MakeVector (Utilities|Array|Get(acopy) (.PropertyValues (Utilities|Struct|BreakLiveLinkBaseFrameData (.FrameData (Utilities|Struct|BreakLiveLinkBasicBlueprintData _dataresult_4))))) (Utilities|Array|Get(acopy) (.PropertyValues (Utilities|Struct|BreakLiveLinkBaseFrameData (.FrameData (Utilities|Struct|BreakLiveLinkBasicBlueprintData _dataresult_5))))) (Utilities|Array|Get(acopy) (.PropertyValues (Utilities|Struct|BreakLiveLinkBaseFrameData (.FrameData (Utilities|Struct|BreakLiveLinkBasicBlueprintData _dataresult_6))))))))))) 0.0 1.0 (.Y (Math|Vector|BreakVector (- (.Location (Math|Transform|BreakTransform (.Transform (Utilities|Struct|BreakLiveLinkTransformFrameData (.FrameData (Utilities|Struct|BreakLiveLinkTransformBlueprintData _dataresult_7)))))) (* (.Scale (Math|Transform|BreakTransform (.Transform (Utilities|Struct|BreakLiveLinkTransformFrameData (.FrameData (Utilities|Struct|BreakLiveLinkTransformBlueprintData _dataresult_7)))))) "0.500000,0.500000,0.500000")))) (.Y (Math|Vector|BreakVector (+ (.Location (Math|Transform|BreakTransform (.Transform (Utilities|Struct|BreakLiveLinkTransformFrameData (.FrameData (Utilities|Struct|BreakLiveLinkTransformBlueprintData _dataresult_7)))))) (* (.Scale (Math|Transform|BreakTransform (.Transform (Utilities|Struct|BreakLiveLinkTransformFrameData (.FrameData (Utilities|Struct|BreakLiveLinkTransformBlueprintData _dataresult_7)))))) "0.500000,0.500000,0.500000"))))) (Math|Float|MapRangeClamped (.Z (Math|Vector|BreakVector (Math|Vector|MakeVector (.Y (Math|Vector|BreakVector (Math|Vector|MakeVector (Utilities|Array|Get(acopy) (.PropertyValues (Utilities|Struct|BreakLiveLinkBaseFrameData (.FrameData (Utilities|Struct|BreakLiveLinkBasicBlueprintData _dataresult_4))))) (Utilities|Array|Get(acopy) (.PropertyValues (Utilities|Struct|BreakLiveLinkBaseFrameData (.FrameData (Utilities|Struct|BreakLiveLinkBasicBlueprintData _dataresult_5))))) (Utilities|Array|Get(acopy) (.PropertyValues (Utilities|Struct|BreakLiveLinkBaseFrameData (.FrameData (Utilities|Struct|BreakLiveLinkBasicBlueprintData _dataresult_6)))))))) (.Z (Math|Vector|BreakVector (Math|Vector|MakeVector (Utilities|Array|Get(acopy) (.PropertyValues (Utilities|Struct|BreakLiveLinkBaseFrameData (.FrameData (Utilities|Struct|BreakLiveLinkBasicBlueprintData _dataresult_4))))) (Utilities|Array|Get(acopy) (.PropertyValues (Utilities|Struct|BreakLiveLinkBaseFrameData (.FrameData (Utilities|Struct|BreakLiveLinkBasicBlueprintData _dataresult_5))))) (Utilities|Array|Get(acopy) (.PropertyValues (Utilities|Struct|BreakLiveLinkBaseFrameData (.FrameData (Utilities|Struct|BreakLiveLinkBasicBlueprintData _dataresult_6)))))))) (.X (Math|Vector|BreakVector (Math|Vector|MakeVector (Utilities|Array|Get(acopy) (.PropertyValues (Utilities|Struct|BreakLiveLinkBaseFrameData (.FrameData (Utilities|Struct|BreakLiveLinkBasicBlueprintData _dataresult_4))))) (Utilities|Array|Get(acopy) (.PropertyValues (Utilities|Struct|BreakLiveLinkBaseFrameData (.FrameData (Utilities|Struct|BreakLiveLinkBasicBlueprintData _dataresult_5))))) (Utilities|Array|Get(acopy) (.PropertyValues (Utilities|Struct|BreakLiveLinkBaseFrameData (.FrameData (Utilities|Struct|BreakLiveLinkBasicBlueprintData _dataresult_6))))))))))) 0.0 1.0 (.Z (Math|Vector|BreakVector (- (.Location (Math|Transform|BreakTransform (.Transform (Utilities|Struct|BreakLiveLinkTransformFrameData (.FrameData (Utilities|Struct|BreakLiveLinkTransformBlueprintData _dataresult_7)))))) (* (.Scale (Math|Transform|BreakTransform (.Transform (Utilities|Struct|BreakLiveLinkTransformFrameData (.FrameData (Utilities|Struct|BreakLiveLinkTransformBlueprintData _dataresult_7)))))) "0.500000,0.500000,0.500000")))) (.Z (Math|Vector|BreakVector (+ (.Location (Math|Transform|BreakTransform (.Transform (Utilities|Struct|BreakLiveLinkTransformFrameData (.FrameData (Utilities|Struct|BreakLiveLinkTransformBlueprintData _dataresult_7)))))) (* (.Scale (Math|Transform|BreakTransform (.Transform (Utilities|Struct|BreakLiveLinkTransformFrameData (.FrameData (Utilities|Struct|BreakLiveLinkTransformBlueprintData _dataresult_7)))))) "0.500000,0.500000,0.500000"))))))))))
            (:then_1
              (if (Variables|Default|GetLog%20Incoming)
                (Development|PrintString (Utilities|String|ToString(Transform) (Math|Transform|MakeTransform (/ (+ (Math|Vector|MakeVector (Math|Float|MapRangeClamped (.X (Math|Vector|BreakVector (Math|Vector|MakeVector (.Y (Math|Vector|BreakVector (Math|Vector|MakeVector (Utilities|Array|Get(acopy) (.PropertyValues (Utilities|Struct|BreakLiveLinkBaseFrameData (.FrameData (Utilities|Struct|BreakLiveLinkBasicBlueprintData _dataresult))))) (Utilities|Array|Get(acopy) (.PropertyValues (Utilities|Struct|BreakLiveLinkBaseFrameData (.FrameData (Utilities|Struct|BreakLiveLinkBasicBlueprintData _dataresult_2))))) (Utilities|Array|Get(acopy) (.PropertyValues (Utilities|Struct|BreakLiveLinkBaseFrameData (.FrameData (Utilities|Struct|BreakLiveLinkBasicBlueprintData _dataresult_3)))))))) (.Z (Math|Vector|BreakVector (Math|Vector|MakeVector (Utilities|Array|Get(acopy) (.PropertyValues (Utilities|Struct|BreakLiveLinkBaseFrameData (.FrameData (Utilities|Struct|BreakLiveLinkBasicBlueprintData _dataresult))))) (Utilities|Array|Get(acopy) (.PropertyValues (Utilities|Struct|BreakLiveLinkBaseFrameData (.FrameData (Utilities|Struct|BreakLiveLinkBasicBlueprintData _dataresult_2))))) (Utilities|Array|Get(acopy) (.PropertyValues (Utilities|Struct|BreakLiveLinkBaseFrameData (.FrameData (Utilities|Struct|BreakLiveLinkBasicBlueprintData _dataresult_3)))))))) (.X (Math|Vector|BreakVector (Math|Vector|MakeVector (Utilities|Array|Get(acopy) (.PropertyValues (Utilities|Struct|BreakLiveLinkBaseFrameData (.FrameData (Utilities|Struct|BreakLiveLinkBasicBlueprintData _dataresult))))) (Utilities|Array|Get(acopy) (.PropertyValues (Utilities|Struct|BreakLiveLinkBaseFrameData (.FrameData (Utilities|Struct|BreakLiveLinkBasicBlueprintData _dataresult_2))))) (Utilities|Array|Get(acopy) (.PropertyValues (Utilities|Struct|BreakLiveLinkBaseFrameData (.FrameData (Utilities|Struct|BreakLiveLinkBasicBlueprintData _dataresult_3))))))))))) 0.0 1.0 (.X (Math|Vector|BreakVector (- (.Location (Math|Transform|BreakTransform (.Transform (Utilities|Struct|BreakLiveLinkTransformFrameData (.FrameData (Utilities|Struct|BreakLiveLinkTransformBlueprintData _dataresult_7)))))) (* (.Scale (Math|Transform|BreakTransform (.Transform (Utilities|Struct|BreakLiveLinkTransformFrameData (.FrameData (Utilities|Struct|BreakLiveLinkTransformBlueprintData _dataresult_7)))))) "0.500000,0.500000,0.500000")))) (.X (Math|Vector|BreakVector (+ (.Location (Math|Transform|BreakTransform (.Transform (Utilities|Struct|BreakLiveLinkTransformFrameData (.FrameData (Utilities|Struct|BreakLiveLinkTransformBlueprintData _dataresult_7)))))) (* (.Scale (Math|Transform|BreakTransform (.Transform (Utilities|Struct|BreakLiveLinkTransformFrameData (.FrameData (Utilities|Struct|BreakLiveLinkTransformBlueprintData _dataresult_7)))))) "0.500000,0.500000,0.500000"))))) (Math|Float|MapRangeClamped (.Y (Math|Vector|BreakVector (Math|Vector|MakeVector (.Y (Math|Vector|BreakVector (Math|Vector|MakeVector (Utilities|Array|Get(acopy) (.PropertyValues (Utilities|Struct|BreakLiveLinkBaseFrameData (.FrameData (Utilities|Struct|BreakLiveLinkBasicBlueprintData _dataresult))))) (Utilities|Array|Get(acopy) (.PropertyValues (Utilities|Struct|BreakLiveLinkBaseFrameData (.FrameData (Utilities|Struct|BreakLiveLinkBasicBlueprintData _dataresult_2))))) (Utilities|Array|Get(acopy) (.PropertyValues (Utilities|Struct|BreakLiveLinkBaseFrameData (.FrameData (Utilities|Struct|BreakLiveLinkBasicBlueprintData _dataresult_3)))))))) (.Z (Math|Vector|BreakVector (Math|Vector|MakeVector (Utilities|Array|Get(acopy) (.PropertyValues (Utilities|Struct|BreakLiveLinkBaseFrameData (.FrameData (Utilities|Struct|BreakLiveLinkBasicBlueprintData _dataresult))))) (Utilities|Array|Get(acopy) (.PropertyValues (Utilities|Struct|BreakLiveLinkBaseFrameData (.FrameData (Utilities|Struct|BreakLiveLinkBasicBlueprintData _dataresult_2))))) (Utilities|Array|Get(acopy) (.PropertyValues (Utilities|Struct|BreakLiveLinkBaseFrameData (.FrameData (Utilities|Struct|BreakLiveLinkBasicBlueprintData _dataresult_3)))))))) (.X (Math|Vector|BreakVector (Math|Vector|MakeVector (Utilities|Array|Get(acopy) (.PropertyValues (Utilities|Struct|BreakLiveLinkBaseFrameData (.FrameData (Utilities|Struct|BreakLiveLinkBasicBlueprintData _dataresult))))) (Utilities|Array|Get(acopy) (.PropertyValues (Utilities|Struct|BreakLiveLinkBaseFrameData (.FrameData (Utilities|Struct|BreakLiveLinkBasicBlueprintData _dataresult_2))))) (Utilities|Array|Get(acopy) (.PropertyValues (Utilities|Struct|BreakLiveLinkBaseFrameData (.FrameData (Utilities|Struct|BreakLiveLinkBasicBlueprintData _dataresult_3))))))))))) 0.0 1.0 (.Y (Math|Vector|BreakVector (- (.Location (Math|Transform|BreakTransform (.Transform (Utilities|Struct|BreakLiveLinkTransformFrameData (.FrameData (Utilities|Struct|BreakLiveLinkTransformBlueprintData _dataresult_7)))))) (* (.Scale (Math|Transform|BreakTransform (.Transform (Utilities|Struct|BreakLiveLinkTransformFrameData (.FrameData (Utilities|Struct|BreakLiveLinkTransformBlueprintData _dataresult_7)))))) "0.500000,0.500000,0.500000")))) (.Y (Math|Vector|BreakVector (+ (.Location (Math|Transform|BreakTransform (.Transform (Utilities|Struct|BreakLiveLinkTransformFrameData (.FrameData (Utilities|Struct|BreakLiveLinkTransformBlueprintData _dataresult_7)))))) (* (.Scale (Math|Transform|BreakTransform (.Transform (Utilities|Struct|BreakLiveLinkTransformFrameData (.FrameData (Utilities|Struct|BreakLiveLinkTransformBlueprintData _dataresult_7)))))) "0.500000,0.500000,0.500000"))))) (Math|Float|MapRangeClamped (.Z (Math|Vector|BreakVector (Math|Vector|MakeVector (.Y (Math|Vector|BreakVector (Math|Vector|MakeVector (Utilities|Array|Get(acopy) (.PropertyValues (Utilities|Struct|BreakLiveLinkBaseFrameData (.FrameData (Utilities|Struct|BreakLiveLinkBasicBlueprintData _dataresult))))) (Utilities|Array|Get(acopy) (.PropertyValues (Utilities|Struct|BreakLiveLinkBaseFrameData (.FrameData (Utilities|Struct|BreakLiveLinkBasicBlueprintData _dataresult_2))))) (Utilities|Array|Get(acopy) (.PropertyValues (Utilities|Struct|BreakLiveLinkBaseFrameData (.FrameData (Utilities|Struct|BreakLiveLinkBasicBlueprintData _dataresult_3)))))))) (.Z (Math|Vector|BreakVector (Math|Vector|MakeVector (Utilities|Array|Get(acopy) (.PropertyValues (Utilities|Struct|BreakLiveLinkBaseFrameData (.FrameData (Utilities|Struct|BreakLiveLinkBasicBlueprintData _dataresult))))) (Utilities|Array|Get(acopy) (.PropertyValues (Utilities|Struct|BreakLiveLinkBaseFrameData (.FrameData (Utilities|Struct|BreakLiveLinkBasicBlueprintData _dataresult_2))))) (Utilities|Array|Get(acopy) (.PropertyValues (Utilities|Struct|BreakLiveLinkBaseFrameData (.FrameData (Utilities|Struct|BreakLiveLinkBasicBlueprintData _dataresult_3)))))))) (.X (Math|Vector|BreakVector (Math|Vector|MakeVector (Utilities|Array|Get(acopy) (.PropertyValues (Utilities|Struct|BreakLiveLinkBaseFrameData (.FrameData (Utilities|Struct|BreakLiveLinkBasicBlueprintData _dataresult))))) (Utilities|Array|Get(acopy) (.PropertyValues (Utilities|Struct|BreakLiveLinkBaseFrameData (.FrameData (Utilities|Struct|BreakLiveLinkBasicBlueprintData _dataresult_2))))) (Utilities|Array|Get(acopy) (.PropertyValues (Utilities|Struct|BreakLiveLinkBaseFrameData (.FrameData (Utilities|Struct|BreakLiveLinkBasicBlueprintData _dataresult_3))))))))))) 0.0 1.0 (.Z (Math|Vector|BreakVector (- (.Location (Math|Transform|BreakTransform (.Transform (Utilities|Struct|BreakLiveLinkTransformFrameData (.FrameData (Utilities|Struct|BreakLiveLinkTransformBlueprintData _dataresult_7)))))) (* (.Scale (Math|Transform|BreakTransform (.Transform (Utilities|Struct|BreakLiveLinkTransformFrameData (.FrameData (Utilities|Struct|BreakLiveLinkTransformBlueprintData _dataresult_7)))))) "0.500000,0.500000,0.500000")))) (.Z (Math|Vector|BreakVector (+ (.Location (Math|Transform|BreakTransform (.Transform (Utilities|Struct|BreakLiveLinkTransformFrameData (.FrameData (Utilities|Struct|BreakLiveLinkTransformBlueprintData _dataresult_7)))))) (* (.Scale (Math|Transform|BreakTransform (.Transform (Utilities|Struct|BreakLiveLinkTransformFrameData (.FrameData (Utilities|Struct|BreakLiveLinkTransformBlueprintData _dataresult_7)))))) "0.500000,0.500000,0.500000")))))) (Math|Vector|MakeVector (Math|Float|MapRangeClamped (.X (Math|Vector|BreakVector (Math|Vector|MakeVector (.Y (Math|Vector|BreakVector (Math|Vector|MakeVector (Utilities|Array|Get(acopy) (.PropertyValues (Utilities|Struct|BreakLiveLinkBaseFrameData (.FrameData (Utilities|Struct|BreakLiveLinkBasicBlueprintData _dataresult_4))))) (Utilities|Array|Get(acopy) (.PropertyValues (Utilities|Struct|BreakLiveLinkBaseFrameData (.FrameData (Utilities|Struct|BreakLiveLinkBasicBlueprintData _dataresult_5))))) (Utilities|Array|Get(acopy) (.PropertyValues (Utilities|Struct|BreakLiveLinkBaseFrameData (.FrameData (Utilities|Struct|BreakLiveLinkBasicBlueprintData _dataresult_6)))))))) (.Z (Math|Vector|BreakVector (Math|Vector|MakeVector (Utilities|Array|Get(acopy) (.PropertyValues (Utilities|Struct|BreakLiveLinkBaseFrameData (.FrameData (Utilities|Struct|BreakLiveLinkBasicBlueprintData _dataresult_4))))) (Utilities|Array|Get(acopy) (.PropertyValues (Utilities|Struct|BreakLiveLinkBaseFrameData (.FrameData (Utilities|Struct|BreakLiveLinkBasicBlueprintData _dataresult_5))))) (Utilities|Array|Get(acopy) (.PropertyValues (Utilities|Struct|BreakLiveLinkBaseFrameData (.FrameData (Utilities|Struct|BreakLiveLinkBasicBlueprintData _dataresult_6)))))))) (.X (Math|Vector|BreakVector (Math|Vector|MakeVector (Utilities|Array|Get(acopy) (.PropertyValues (Utilities|Struct|BreakLiveLinkBaseFrameData (.FrameData (Utilities|Struct|BreakLiveLinkBasicBlueprintData _dataresult_4))))) (Utilities|Array|Get(acopy) (.PropertyValues (Utilities|Struct|BreakLiveLinkBaseFrameData (.FrameData (Utilities|Struct|BreakLiveLinkBasicBlueprintData _dataresult_5))))) (Utilities|Array|Get(acopy) (.PropertyValues (Utilities|Struct|BreakLiveLinkBaseFrameData (.FrameData (Utilities|Struct|BreakLiveLinkBasicBlueprintData _dataresult_6))))))))))) 0.0 1.0 (.X (Math|Vector|BreakVector (- (.Location (Math|Transform|BreakTransform (.Transform (Utilities|Struct|BreakLiveLinkTransformFrameData (.FrameData (Utilities|Struct|BreakLiveLinkTransformBlueprintData _dataresult_7)))))) (* (.Scale (Math|Transform|BreakTransform (.Transform (Utilities|Struct|BreakLiveLinkTransformFrameData (.FrameData (Utilities|Struct|BreakLiveLinkTransformBlueprintData _dataresult_7)))))) "0.500000,0.500000,0.500000")))) (.X (Math|Vector|BreakVector (+ (.Location (Math|Transform|BreakTransform (.Transform (Utilities|Struct|BreakLiveLinkTransformFrameData (.FrameData (Utilities|Struct|BreakLiveLinkTransformBlueprintData _dataresult_7)))))) (* (.Scale (Math|Transform|BreakTransform (.Transform (Utilities|Struct|BreakLiveLinkTransformFrameData (.FrameData (Utilities|Struct|BreakLiveLinkTransformBlueprintData _dataresult_7)))))) "0.500000,0.500000,0.500000"))))) (Math|Float|MapRangeClamped (.Y (Math|Vector|BreakVector (Math|Vector|MakeVector (.Y (Math|Vector|BreakVector (Math|Vector|MakeVector (Utilities|Array|Get(acopy) (.PropertyValues (Utilities|Struct|BreakLiveLinkBaseFrameData (.FrameData (Utilities|Struct|BreakLiveLinkBasicBlueprintData _dataresult_4))))) (Utilities|Array|Get(acopy) (.PropertyValues (Utilities|Struct|BreakLiveLinkBaseFrameData (.FrameData (Utilities|Struct|BreakLiveLinkBasicBlueprintData _dataresult_5))))) (Utilities|Array|Get(acopy) (.PropertyValues (Utilities|Struct|BreakLiveLinkBaseFrameData (.FrameData (Utilities|Struct|BreakLiveLinkBasicBlueprintData _dataresult_6)))))))) (.Z (Math|Vector|BreakVector (Math|Vector|MakeVector (Utilities|Array|Get(acopy) (.PropertyValues (Utilities|Struct|BreakLiveLinkBaseFrameData (.FrameData (Utilities|Struct|BreakLiveLinkBasicBlueprintData _dataresult_4))))) (Utilities|Array|Get(acopy) (.PropertyValues (Utilities|Struct|BreakLiveLinkBaseFrameData (.FrameData (Utilities|Struct|BreakLiveLinkBasicBlueprintData _dataresult_5))))) (Utilities|Array|Get(acopy) (.PropertyValues (Utilities|Struct|BreakLiveLinkBaseFrameData (.FrameData (Utilities|Struct|BreakLiveLinkBasicBlueprintData _dataresult_6)))))))) (.X (Math|Vector|BreakVector (Math|Vector|MakeVector (Utilities|Array|Get(acopy) (.PropertyValues (Utilities|Struct|BreakLiveLinkBaseFrameData (.FrameData (Utilities|Struct|BreakLiveLinkBasicBlueprintData _dataresult_4))))) (Utilities|Array|Get(acopy) (.PropertyValues (Utilities|Struct|BreakLiveLinkBaseFrameData (.FrameData (Utilities|Struct|BreakLiveLinkBasicBlueprintData _dataresult_5))))) (Utilities|Array|Get(acopy) (.PropertyValues (Utilities|Struct|BreakLiveLinkBaseFrameData (.FrameData (Utilities|Struct|BreakLiveLinkBasicBlueprintData _dataresult_6))))))))))) 0.0 1.0 (.Y (Math|Vector|BreakVector (- (.Location (Math|Transform|BreakTransform (.Transform (Utilities|Struct|BreakLiveLinkTransformFrameData (.FrameData (Utilities|Struct|BreakLiveLinkTransformBlueprintData _dataresult_7)))))) (* (.Scale (Math|Transform|BreakTransform (.Transform (Utilities|Struct|BreakLiveLinkTransformFrameData (.FrameData (Utilities|Struct|BreakLiveLinkTransformBlueprintData _dataresult_7)))))) "0.500000,0.500000,0.500000")))) (.Y (Math|Vector|BreakVector (+ (.Location (Math|Transform|BreakTransform (.Transform (Utilities|Struct|BreakLiveLinkTransformFrameData (.FrameData (Utilities|Struct|BreakLiveLinkTransformBlueprintData _dataresult_7)))))) (* (.Scale (Math|Transform|BreakTransform (.Transform (Utilities|Struct|BreakLiveLinkTransformFrameData (.FrameData (Utilities|Struct|BreakLiveLinkTransformBlueprintData _dataresult_7)))))) "0.500000,0.500000,0.500000"))))) (Math|Float|MapRangeClamped (.Z (Math|Vector|BreakVector (Math|Vector|MakeVector (.Y (Math|Vector|BreakVector (Math|Vector|MakeVector (Utilities|Array|Get(acopy) (.PropertyValues (Utilities|Struct|BreakLiveLinkBaseFrameData (.FrameData (Utilities|Struct|BreakLiveLinkBasicBlueprintData _dataresult_4))))) (Utilities|Array|Get(acopy) (.PropertyValues (Utilities|Struct|BreakLiveLinkBaseFrameData (.FrameData (Utilities|Struct|BreakLiveLinkBasicBlueprintData _dataresult_5))))) (Utilities|Array|Get(acopy) (.PropertyValues (Utilities|Struct|BreakLiveLinkBaseFrameData (.FrameData (Utilities|Struct|BreakLiveLinkBasicBlueprintData _dataresult_6)))))))) (.Z (Math|Vector|BreakVector (Math|Vector|MakeVector (Utilities|Array|Get(acopy) (.PropertyValues (Utilities|Struct|BreakLiveLinkBaseFrameData (.FrameData (Utilities|Struct|BreakLiveLinkBasicBlueprintData _dataresult_4))))) (Utilities|Array|Get(acopy) (.PropertyValues (Utilities|Struct|BreakLiveLinkBaseFrameData (.FrameData (Utilities|Struct|BreakLiveLinkBasicBlueprintData _dataresult_5))))) (Utilities|Array|Get(acopy) (.PropertyValues (Utilities|Struct|BreakLiveLinkBaseFrameData (.FrameData (Utilities|Struct|BreakLiveLinkBasicBlueprintData _dataresult_6)))))))) (.X (Math|Vector|BreakVector (Math|Vector|MakeVector (Utilities|Array|Get(acopy) (.PropertyValues (Utilities|Struct|BreakLiveLinkBaseFrameData (.FrameData (Utilities|Struct|BreakLiveLinkBasicBlueprintData _dataresult_4))))) (Utilities|Array|Get(acopy) (.PropertyValues (Utilities|Struct|BreakLiveLinkBaseFrameData (.FrameData (Utilities|Struct|BreakLiveLinkBasicBlueprintData _dataresult_5))))) (Utilities|Array|Get(acopy) (.PropertyValues (Utilities|Struct|BreakLiveLinkBaseFrameData (.FrameData (Utilities|Struct|BreakLiveLinkBasicBlueprintData _dataresult_6))))))))))) 0.0 1.0 (.Z (Math|Vector|BreakVector (- (.Location (Math|Transform|BreakTransform (.Transform (Utilities|Struct|BreakLiveLinkTransformFrameData (.FrameData (Utilities|Struct|BreakLiveLinkTransformBlueprintData _dataresult_7)))))) (* (.Scale (Math|Transform|BreakTransform (.Transform (Utilities|Struct|BreakLiveLinkTransformFrameData (.FrameData (Utilities|Struct|BreakLiveLinkTransformBlueprintData _dataresult_7)))))) "0.500000,0.500000,0.500000")))) (.Z (Math|Vector|BreakVector (+ (.Location (Math|Transform|BreakTransform (.Transform (Utilities|Struct|BreakLiveLinkTransformFrameData (.FrameData (Utilities|Struct|BreakLiveLinkTransformBlueprintData _dataresult_7)))))) (* (.Scale (Math|Transform|BreakTransform (.Transform (Utilities|Struct|BreakLiveLinkTransformFrameData (.FrameData (Utilities|Struct|BreakLiveLinkTransformBlueprintData _dataresult_7)))))) "0.500000,0.500000,0.500000"))))))) "2.000000,2.000000,2.000000") "0, 0, 0" (- (Math|Vector|MakeVector (Math|Float|MapRangeClamped (.X (Math|Vector|BreakVector (Math|Vector|MakeVector (.Y (Math|Vector|BreakVector (Math|Vector|MakeVector (Utilities|Array|Get(acopy) (.PropertyValues (Utilities|Struct|BreakLiveLinkBaseFrameData (.FrameData (Utilities|Struct|BreakLiveLinkBasicBlueprintData _dataresult))))) (Utilities|Array|Get(acopy) (.PropertyValues (Utilities|Struct|BreakLiveLinkBaseFrameData (.FrameData (Utilities|Struct|BreakLiveLinkBasicBlueprintData _dataresult_2))))) (Utilities|Array|Get(acopy) (.PropertyValues (Utilities|Struct|BreakLiveLinkBaseFrameData (.FrameData (Utilities|Struct|BreakLiveLinkBasicBlueprintData _dataresult_3)))))))) (.Z (Math|Vector|BreakVector (Math|Vector|MakeVector (Utilities|Array|Get(acopy) (.PropertyValues (Utilities|Struct|BreakLiveLinkBaseFrameData (.FrameData (Utilities|Struct|BreakLiveLinkBasicBlueprintData _dataresult))))) (Utilities|Array|Get(acopy) (.PropertyValues (Utilities|Struct|BreakLiveLinkBaseFrameData (.FrameData (Utilities|Struct|BreakLiveLinkBasicBlueprintData _dataresult_2))))) (Utilities|Array|Get(acopy) (.PropertyValues (Utilities|Struct|BreakLiveLinkBaseFrameData (.FrameData (Utilities|Struct|BreakLiveLinkBasicBlueprintData _dataresult_3)))))))) (.X (Math|Vector|BreakVector (Math|Vector|MakeVector (Utilities|Array|Get(acopy) (.PropertyValues (Utilities|Struct|BreakLiveLinkBaseFrameData (.FrameData (Utilities|Struct|BreakLiveLinkBasicBlueprintData _dataresult))))) (Utilities|Array|Get(acopy) (.PropertyValues (Utilities|Struct|BreakLiveLinkBaseFrameData (.FrameData (Utilities|Struct|BreakLiveLinkBasicBlueprintData _dataresult_2))))) (Utilities|Array|Get(acopy) (.PropertyValues (Utilities|Struct|BreakLiveLinkBaseFrameData (.FrameData (Utilities|Struct|BreakLiveLinkBasicBlueprintData _dataresult_3))))))))))) 0.0 1.0 (.X (Math|Vector|BreakVector (- (.Location (Math|Transform|BreakTransform (.Transform (Utilities|Struct|BreakLiveLinkTransformFrameData (.FrameData (Utilities|Struct|BreakLiveLinkTransformBlueprintData _dataresult_7)))))) (* (.Scale (Math|Transform|BreakTransform (.Transform (Utilities|Struct|BreakLiveLinkTransformFrameData (.FrameData (Utilities|Struct|BreakLiveLinkTransformBlueprintData _dataresult_7)))))) "0.500000,0.500000,0.500000")))) (.X (Math|Vector|BreakVector (+ (.Location (Math|Transform|BreakTransform (.Transform (Utilities|Struct|BreakLiveLinkTransformFrameData (.FrameData (Utilities|Struct|BreakLiveLinkTransformBlueprintData _dataresult_7)))))) (* (.Scale (Math|Transform|BreakTransform (.Transform (Utilities|Struct|BreakLiveLinkTransformFrameData (.FrameData (Utilities|Struct|BreakLiveLinkTransformBlueprintData _dataresult_7)))))) "0.500000,0.500000,0.500000"))))) (Math|Float|MapRangeClamped (.Y (Math|Vector|BreakVector (Math|Vector|MakeVector (.Y (Math|Vector|BreakVector (Math|Vector|MakeVector (Utilities|Array|Get(acopy) (.PropertyValues (Utilities|Struct|BreakLiveLinkBaseFrameData (.FrameData (Utilities|Struct|BreakLiveLinkBasicBlueprintData _dataresult))))) (Utilities|Array|Get(acopy) (.PropertyValues (Utilities|Struct|BreakLiveLinkBaseFrameData (.FrameData (Utilities|Struct|BreakLiveLinkBasicBlueprintData _dataresult_2))))) (Utilities|Array|Get(acopy) (.PropertyValues (Utilities|Struct|BreakLiveLinkBaseFrameData (.FrameData (Utilities|Struct|BreakLiveLinkBasicBlueprintData _dataresult_3)))))))) (.Z (Math|Vector|BreakVector (Math|Vector|MakeVector (Utilities|Array|Get(acopy) (.PropertyValues (Utilities|Struct|BreakLiveLinkBaseFrameData (.FrameData (Utilities|Struct|BreakLiveLinkBasicBlueprintData _dataresult))))) (Utilities|Array|Get(acopy) (.PropertyValues (Utilities|Struct|BreakLiveLinkBaseFrameData (.FrameData (Utilities|Struct|BreakLiveLinkBasicBlueprintData _dataresult_2))))) (Utilities|Array|Get(acopy) (.PropertyValues (Utilities|Struct|BreakLiveLinkBaseFrameData (.FrameData (Utilities|Struct|BreakLiveLinkBasicBlueprintData _dataresult_3)))))))) (.X (Math|Vector|BreakVector (Math|Vector|MakeVector (Utilities|Array|Get(acopy) (.PropertyValues (Utilities|Struct|BreakLiveLinkBaseFrameData (.FrameData (Utilities|Struct|BreakLiveLinkBasicBlueprintData _dataresult))))) (Utilities|Array|Get(acopy) (.PropertyValues (Utilities|Struct|BreakLiveLinkBaseFrameData (.FrameData (Utilities|Struct|BreakLiveLinkBasicBlueprintData _dataresult_2))))) (Utilities|Array|Get(acopy) (.PropertyValues (Utilities|Struct|BreakLiveLinkBaseFrameData (.FrameData (Utilities|Struct|BreakLiveLinkBasicBlueprintData _dataresult_3))))))))))) 0.0 1.0 (.Y (Math|Vector|BreakVector (- (.Location (Math|Transform|BreakTransform (.Transform (Utilities|Struct|BreakLiveLinkTransformFrameData (.FrameData (Utilities|Struct|BreakLiveLinkTransformBlueprintData _dataresult_7)))))) (* (.Scale (Math|Transform|BreakTransform (.Transform (Utilities|Struct|BreakLiveLinkTransformFrameData (.FrameData (Utilities|Struct|BreakLiveLinkTransformBlueprintData _dataresult_7)))))) "0.500000,0.500000,0.500000")))) (.Y (Math|Vector|BreakVector (+ (.Location (Math|Transform|BreakTransform (.Transform (Utilities|Struct|BreakLiveLinkTransformFrameData (.FrameData (Utilities|Struct|BreakLiveLinkTransformBlueprintData _dataresult_7)))))) (* (.Scale (Math|Transform|BreakTransform (.Transform (Utilities|Struct|BreakLiveLinkTransformFrameData (.FrameData (Utilities|Struct|BreakLiveLinkTransformBlueprintData _dataresult_7)))))) "0.500000,0.500000,0.500000"))))) (Math|Float|MapRangeClamped (.Z (Math|Vector|BreakVector (Math|Vector|MakeVector (.Y (Math|Vector|BreakVector (Math|Vector|MakeVector (Utilities|Array|Get(acopy) (.PropertyValues (Utilities|Struct|BreakLiveLinkBaseFrameData (.FrameData (Utilities|Struct|BreakLiveLinkBasicBlueprintData _dataresult))))) (Utilities|Array|Get(acopy) (.PropertyValues (Utilities|Struct|BreakLiveLinkBaseFrameData (.FrameData (Utilities|Struct|BreakLiveLinkBasicBlueprintData _dataresult_2))))) (Utilities|Array|Get(acopy) (.PropertyValues (Utilities|Struct|BreakLiveLinkBaseFrameData (.FrameData (Utilities|Struct|BreakLiveLinkBasicBlueprintData _dataresult_3)))))))) (.Z (Math|Vector|BreakVector (Math|Vector|MakeVector (Utilities|Array|Get(acopy) (.PropertyValues (Utilities|Struct|BreakLiveLinkBaseFrameData (.FrameData (Utilities|Struct|BreakLiveLinkBasicBlueprintData _dataresult))))) (Utilities|Array|Get(acopy) (.PropertyValues (Utilities|Struct|BreakLiveLinkBaseFrameData (.FrameData (Utilities|Struct|BreakLiveLinkBasicBlueprintData _dataresult_2))))) (Utilities|Array|Get(acopy) (.PropertyValues (Utilities|Struct|BreakLiveLinkBaseFrameData (.FrameData (Utilities|Struct|BreakLiveLinkBasicBlueprintData _dataresult_3)))))))) (.X (Math|Vector|BreakVector (Math|Vector|MakeVector (Utilities|Array|Get(acopy) (.PropertyValues (Utilities|Struct|BreakLiveLinkBaseFrameData (.FrameData (Utilities|Struct|BreakLiveLinkBasicBlueprintData _dataresult))))) (Utilities|Array|Get(acopy) (.PropertyValues (Utilities|Struct|BreakLiveLinkBaseFrameData (.FrameData (Utilities|Struct|BreakLiveLinkBasicBlueprintData _dataresult_2))))) (Utilities|Array|Get(acopy) (.PropertyValues (Utilities|Struct|BreakLiveLinkBaseFrameData (.FrameData (Utilities|Struct|BreakLiveLinkBasicBlueprintData _dataresult_3))))))))))) 0.0 1.0 (.Z (Math|Vector|BreakVector (- (.Location (Math|Transform|BreakTransform (.Transform (Utilities|Struct|BreakLiveLinkTransformFrameData (.FrameData (Utilities|Struct|BreakLiveLinkTransformBlueprintData _dataresult_7)))))) (* (.Scale (Math|Transform|BreakTransform (.Transform (Utilities|Struct|BreakLiveLinkTransformFrameData (.FrameData (Utilities|Struct|BreakLiveLinkTransformBlueprintData _dataresult_7)))))) "0.500000,0.500000,0.500000")))) (.Z (Math|Vector|BreakVector (+ (.Location (Math|Transform|BreakTransform (.Transform (Utilities|Struct|BreakLiveLinkTransformFrameData (.FrameData (Utilities|Struct|BreakLiveLinkTransformBlueprintData _dataresult_7)))))) (* (.Scale (Math|Transform|BreakTransform (.Transform (Utilities|Struct|BreakLiveLinkTransformFrameData (.FrameData (Utilities|Struct|BreakLiveLinkTransformBlueprintData _dataresult_7)))))) "0.500000,0.500000,0.500000")))))) (Math|Vector|MakeVector (Math|Float|MapRangeClamped (.X (Math|Vector|BreakVector (Math|Vector|MakeVector (.Y (Math|Vector|BreakVector (Math|Vector|MakeVector (Utilities|Array|Get(acopy) (.PropertyValues (Utilities|Struct|BreakLiveLinkBaseFrameData (.FrameData (Utilities|Struct|BreakLiveLinkBasicBlueprintData _dataresult_4))))) (Utilities|Array|Get(acopy) (.PropertyValues (Utilities|Struct|BreakLiveLinkBaseFrameData (.FrameData (Utilities|Struct|BreakLiveLinkBasicBlueprintData _dataresult_5))))) (Utilities|Array|Get(acopy) (.PropertyValues (Utilities|Struct|BreakLiveLinkBaseFrameData (.FrameData (Utilities|Struct|BreakLiveLinkBasicBlueprintData _dataresult_6)))))))) (.Z (Math|Vector|BreakVector (Math|Vector|MakeVector (Utilities|Array|Get(acopy) (.PropertyValues (Utilities|Struct|BreakLiveLinkBaseFrameData (.FrameData (Utilities|Struct|BreakLiveLinkBasicBlueprintData _dataresult_4))))) (Utilities|Array|Get(acopy) (.PropertyValues (Utilities|Struct|BreakLiveLinkBaseFrameData (.FrameData (Utilities|Struct|BreakLiveLinkBasicBlueprintData _dataresult_5))))) (Utilities|Array|Get(acopy) (.PropertyValues (Utilities|Struct|BreakLiveLinkBaseFrameData (.FrameData (Utilities|Struct|BreakLiveLinkBasicBlueprintData _dataresult_6)))))))) (.X (Math|Vector|BreakVector (Math|Vector|MakeVector (Utilities|Array|Get(acopy) (.PropertyValues (Utilities|Struct|BreakLiveLinkBaseFrameData (.FrameData (Utilities|Struct|BreakLiveLinkBasicBlueprintData _dataresult_4))))) (Utilities|Array|Get(acopy) (.PropertyValues (Utilities|Struct|BreakLiveLinkBaseFrameData (.FrameData (Utilities|Struct|BreakLiveLinkBasicBlueprintData _dataresult_5))))) (Utilities|Array|Get(acopy) (.PropertyValues (Utilities|Struct|BreakLiveLinkBaseFrameData (.FrameData (Utilities|Struct|BreakLiveLinkBasicBlueprintData _dataresult_6))))))))))) 0.0 1.0 (.X (Math|Vector|BreakVector (- (.Location (Math|Transform|BreakTransform (.Transform (Utilities|Struct|BreakLiveLinkTransformFrameData (.FrameData (Utilities|Struct|BreakLiveLinkTransformBlueprintData _dataresult_7)))))) (* (.Scale (Math|Transform|BreakTransform (.Transform (Utilities|Struct|BreakLiveLinkTransformFrameData (.FrameData (Utilities|Struct|BreakLiveLinkTransformBlueprintData _dataresult_7)))))) "0.500000,0.500000,0.500000")))) (.X (Math|Vector|BreakVector (+ (.Location (Math|Transform|BreakTransform (.Transform (Utilities|Struct|BreakLiveLinkTransformFrameData (.FrameData (Utilities|Struct|BreakLiveLinkTransformBlueprintData _dataresult_7)))))) (* (.Scale (Math|Transform|BreakTransform (.Transform (Utilities|Struct|BreakLiveLinkTransformFrameData (.FrameData (Utilities|Struct|BreakLiveLinkTransformBlueprintData _dataresult_7)))))) "0.500000,0.500000,0.500000"))))) (Math|Float|MapRangeClamped (.Y (Math|Vector|BreakVector (Math|Vector|MakeVector (.Y (Math|Vector|BreakVector (Math|Vector|MakeVector (Utilities|Array|Get(acopy) (.PropertyValues (Utilities|Struct|BreakLiveLinkBaseFrameData (.FrameData (Utilities|Struct|BreakLiveLinkBasicBlueprintData _dataresult_4))))) (Utilities|Array|Get(acopy) (.PropertyValues (Utilities|Struct|BreakLiveLinkBaseFrameData (.FrameData (Utilities|Struct|BreakLiveLinkBasicBlueprintData _dataresult_5))))) (Utilities|Array|Get(acopy) (.PropertyValues (Utilities|Struct|BreakLiveLinkBaseFrameData (.FrameData (Utilities|Struct|BreakLiveLinkBasicBlueprintData _dataresult_6)))))))) (.Z (Math|Vector|BreakVector (Math|Vector|MakeVector (Utilities|Array|Get(acopy) (.PropertyValues (Utilities|Struct|BreakLiveLinkBaseFrameData (.FrameData (Utilities|Struct|BreakLiveLinkBasicBlueprintData _dataresult_4))))) (Utilities|Array|Get(acopy) (.PropertyValues (Utilities|Struct|BreakLiveLinkBaseFrameData (.FrameData (Utilities|Struct|BreakLiveLinkBasicBlueprintData _dataresult_5))))) (Utilities|Array|Get(acopy) (.PropertyValues (Utilities|Struct|BreakLiveLinkBaseFrameData (.FrameData (Utilities|Struct|BreakLiveLinkBasicBlueprintData _dataresult_6)))))))) (.X (Math|Vector|BreakVector (Math|Vector|MakeVector (Utilities|Array|Get(acopy) (.PropertyValues (Utilities|Struct|BreakLiveLinkBaseFrameData (.FrameData (Utilities|Struct|BreakLiveLinkBasicBlueprintData _dataresult_4))))) (Utilities|Array|Get(acopy) (.PropertyValues (Utilities|Struct|BreakLiveLinkBaseFrameData (.FrameData (Utilities|Struct|BreakLiveLinkBasicBlueprintData _dataresult_5))))) (Utilities|Array|Get(acopy) (.PropertyValues (Utilities|Struct|BreakLiveLinkBaseFrameData (.FrameData (Utilities|Struct|BreakLiveLinkBasicBlueprintData _dataresult_6))))))))))) 0.0 1.0 (.Y (Math|Vector|BreakVector (- (.Location (Math|Transform|BreakTransform (.Transform (Utilities|Struct|BreakLiveLinkTransformFrameData (.FrameData (Utilities|Struct|BreakLiveLinkTransformBlueprintData _dataresult_7)))))) (* (.Scale (Math|Transform|BreakTransform (.Transform (Utilities|Struct|BreakLiveLinkTransformFrameData (.FrameData (Utilities|Struct|BreakLiveLinkTransformBlueprintData _dataresult_7)))))) "0.500000,0.500000,0.500000")))) (.Y (Math|Vector|BreakVector (+ (.Location (Math|Transform|BreakTransform (.Transform (Utilities|Struct|BreakLiveLinkTransformFrameData (.FrameData (Utilities|Struct|BreakLiveLinkTransformBlueprintData _dataresult_7)))))) (* (.Scale (Math|Transform|BreakTransform (.Transform (Utilities|Struct|BreakLiveLinkTransformFrameData (.FrameData (Utilities|Struct|BreakLiveLinkTransformBlueprintData _dataresult_7)))))) "0.500000,0.500000,0.500000"))))) (Math|Float|MapRangeClamped (.Z (Math|Vector|BreakVector (Math|Vector|MakeVector (.Y (Math|Vector|BreakVector (Math|Vector|MakeVector (Utilities|Array|Get(acopy) (.PropertyValues (Utilities|Struct|BreakLiveLinkBaseFrameData (.FrameData (Utilities|Struct|BreakLiveLinkBasicBlueprintData _dataresult_4))))) (Utilities|Array|Get(acopy) (.PropertyValues (Utilities|Struct|BreakLiveLinkBaseFrameData (.FrameData (Utilities|Struct|BreakLiveLinkBasicBlueprintData _dataresult_5))))) (Utilities|Array|Get(acopy) (.PropertyValues (Utilities|Struct|BreakLiveLinkBaseFrameData (.FrameData (Utilities|Struct|BreakLiveLinkBasicBlueprintData _dataresult_6)))))))) (.Z (Math|Vector|BreakVector (Math|Vector|MakeVector (Utilities|Array|Get(acopy) (.PropertyValues (Utilities|Struct|BreakLiveLinkBaseFrameData (.FrameData (Utilities|Struct|BreakLiveLinkBasicBlueprintData _dataresult_4))))) (Utilities|Array|Get(acopy) (.PropertyValues (Utilities|Struct|BreakLiveLinkBaseFrameData (.FrameData (Utilities|Struct|BreakLiveLinkBasicBlueprintData _dataresult_5))))) (Utilities|Array|Get(acopy) (.PropertyValues (Utilities|Struct|BreakLiveLinkBaseFrameData (.FrameData (Utilities|Struct|BreakLiveLinkBasicBlueprintData _dataresult_6)))))))) (.X (Math|Vector|BreakVector (Math|Vector|MakeVector (Utilities|Array|Get(acopy) (.PropertyValues (Utilities|Struct|BreakLiveLinkBaseFrameData (.FrameData (Utilities|Struct|BreakLiveLinkBasicBlueprintData _dataresult_4))))) (Utilities|Array|Get(acopy) (.PropertyValues (Utilities|Struct|BreakLiveLinkBaseFrameData (.FrameData (Utilities|Struct|BreakLiveLinkBasicBlueprintData _dataresult_5))))) (Utilities|Array|Get(acopy) (.PropertyValues (Utilities|Struct|BreakLiveLinkBaseFrameData (.FrameData (Utilities|Struct|BreakLiveLinkBasicBlueprintData _dataresult_6))))))))))) 0.0 1.0 (.Z (Math|Vector|BreakVector (- (.Location (Math|Transform|BreakTransform (.Transform (Utilities|Struct|BreakLiveLinkTransformFrameData (.FrameData (Utilities|Struct|BreakLiveLinkTransformBlueprintData _dataresult_7)))))) (* (.Scale (Math|Transform|BreakTransform (.Transform (Utilities|Struct|BreakLiveLinkTransformFrameData (.FrameData (Utilities|Struct|BreakLiveLinkTransformBlueprintData _dataresult_7)))))) "0.500000,0.500000,0.500000")))) (.Z (Math|Vector|BreakVector (+ (.Location (Math|Transform|BreakTransform (.Transform (Utilities|Struct|BreakLiveLinkTransformFrameData (.FrameData (Utilities|Struct|BreakLiveLinkTransformBlueprintData _dataresult_7)))))) (* (.Scale (Math|Transform|BreakTransform (.Transform (Utilities|Struct|BreakLiveLinkTransformFrameData (.FrameData (Utilities|Struct|BreakLiveLinkTransformBlueprintData _dataresult_7)))))) "0.500000,0.500000,0.500000"))))))))) false)))))))))